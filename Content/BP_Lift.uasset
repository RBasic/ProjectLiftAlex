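; Lift actor that carries the first-person player between the bottom and top of a shaft, passing intermediate levels without stopping.
; The construction script builds the shaft, cabin, doors and overlap capsule from NbFloors and the starting end set by LiftUp.
; Entering the capsule closes doors through two chained timelines, reopening them if the player has left.
; Otherwise Tick moves the cabin at constant speed, then flips LiftUp and opens that end's doors.
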(event OnComponentBeginOverlap(OverlapPlayer)
  (params (OverlappedComponent :type Primitive%20Component%20Object%20Reference) (OtherActor :type Actor%20Object%20Reference) (OtherComp :type Primitive%20Component%20Object%20Reference) (OtherBodyIndex :type Integer) (bFromSweep :type Boolean) (SweepResult :type Hit%20Result%20Structure%20%28by%20ref%29))
  (Utilities|Casting|CastToBP_FirstPersonCharacter OtherActor)
  (CallFunction|ManageLiftDoors false))

(event Custom|ManageLiftDoors
  (params (Open :type Boolean))
  (bind _liftdoors (Variables|Default|GetLiftDoors))
  (if Open
    (bind (_direction _newtrack_0) (Timeline|Timeline Reverse)
      (:Update
        (Transformation|SetRelativeRotation (Utilities|Array|Get(acopy) _liftdoors) (Math|Rotator|MakeRotator 0.0 0.0 (* _newtrack_0 3e+01)) false false)
        (Transformation|SetRelativeRotation (Utilities|Array|Get(acopy) _liftdoors 1) (Math|Rotator|MakeRotator 0.0 0.0 (* _newtrack_0 -3e+01)) false false))
      (:ExternalDoors
        (CallFunction|ManageDoors (select (Variables|Default|GetLiftUp) (Variables|Default|GetUpDoors) (Variables|Default|GetDownDoors)) (Utilities|Select :Index _direction :Forward false :Backward true))))
    (else
      (Timeline|Timeline Play))))

(event Custom|ManageDoors
  (params (Doors :type Array%20of%20Static%20Mesh%20Component%20Object%20References) (Open :type Boolean))
  (if Open
    (bind (_direction _newtrack_0) (Timeline|MoveDoors Reverse)
      (:Update
        (Transformation|SetRelativeRotation (Utilities|Array|Get(acopy) Doors) (Math|Rotator|MakeRotator 0.0 0.0 (* _newtrack_0 3e+01)) false false)
        (Transformation|SetRelativeRotation (Utilities|Array|Get(acopy) Doors 1) (Math|Rotator|MakeRotator 0.0 0.0 (* _newtrack_0 -3e+01)) false false))
      (:Finished
        (switch Utilities|FlowControl|Switch|SwitchonETimelineDirection _direction
          (:Forward
            (if (Collision|IsOverlappingActor (Variables|Default|GetOverlapPlayer) (Game|GetPlayerCharacter 0) :!class /Script/Engine.PrimitiveComponent)
              (Variables|Default|SetMove true)
              (else
                (CallFunction|ManageLiftDoors true)))))))
    (else
      (Timeline|MoveDoors Play))))

(event EventBeginPlay)

(event Collision|EventActorBeginOverlap
  (params (OtherActor :type Actor%20Object%20Reference)))

(event EventTick
  (params (DeltaSeconds :type Float%20%28single-precision%29))
  (bind _liftref (Variables|Default|GetLiftRef))
  (if (Variables|Default|GetMove)
    (Transformation|SetRelativeLocation _liftref (Math|Vector|MakeVector 0.0 0.0 (Math|Interpolation|FInterptoConstant (.z (Variables|/Script/Engine.SceneComponent|GetRelativeLocation _liftref)) (select (Variables|Default|GetLiftUp) 0.0 (* (Variables|Default|GetNbFloors) 5e+02)) (Utilities|Time|GetWorldDeltaSeconds) 1e+02)) false false)
    (if (== (.z (Variables|/Script/Engine.SceneComponent|GetRelativeLocation (Variables|Default|GetLiftRef))) (select (Variables|Default|GetLiftUp) 0.0 (* (Variables|Default|GetNbFloors) 5e+02)))
      (Variables|Default|SetMove false)
      (Variables|Default|SetLiftUp (not (Variables|Default|GetLiftUp)))
      (CallFunction|ManageLiftDoors true))))

(fn ConstructionScript
  (Utilities|FlowControl|Sequence
    (:then_0
      ;[1 1 1] Setup Lift
      (bind _returnvalue (AddComponent|AddStaticMeshComponent false (Math|Transform|MakeTransform (Math|Vector|MakeVector 0.0 0.0 (select (Variables|Default|GetLiftUp) (* (Variables|Default|GetNbFloors) 5e+02) 0.0)) "0, 0, 0" "1.000000,1.000000,1.000000")))
      (Variables|Default|SetLiftRef _returnvalue)
      (bind _returnvalue_2 (AddComponent|AddStaticMeshComponent true (Math|Transform|MakeTransform "0.000000,-200.000000,0.000000" "0.000000,-30.000000,0.000000" "1.000000,1.000000,1.000000")))
      (Transformation|AttachComponentToComponent _returnvalue_2 _returnvalue "None" "KeepRelative" "KeepRelative" "SnapToTarget" true)
      (bind _returnvalue_3 (AddComponent|AddStaticMeshComponent true (Math|Transform|MakeTransform "0.000000,-200.000000,0.000000" "0.000000,30.000000,0.000000" "1.000000,1.000000,1.000000")))
      (Transformation|AttachComponentToComponent _returnvalue_3 _returnvalue "None" "KeepRelative" "KeepRelative" "SnapToTarget" true)
      (bind _returnvalue_4 (AddComponent|AddCapsuleComponent true (Math|Transform|MakeTransform (Math|Vector|MakeVector 0.0 -2e+02 1e+02) "0, 0, 0" "1.000000,1.000000,1.000000")))
      (bind _output_get (Variables|Default|SetOverlapPlayer _returnvalue_4))
      (Transformation|AttachComponentToComponent _output_get _returnvalue "None" "KeepRelative" "KeepRelative" "KeepWorld" true)
      (Variables|Default|SetLiftDoors (Utilities|Array|MakeArray _returnvalue_3 _returnvalue_2)))
    (:then_1
      ;[1 1 1] Setup downDoors
      (bind _returnvalue_5 (AddComponent|AddStaticMeshComponent false))
      (bind _returnvalue_6 (AddComponent|AddStaticMeshComponent true (Math|Transform|MakeTransform "0.000000,-200.000000,0.000000" (Math|Rotator|MakeRotator 0.0 0.0 (select (Variables|Default|GetLiftUp) 0.0 -3e+01)) "1.000000,1.000000,1.000000")))
      (Transformation|AttachComponentToComponent _returnvalue_6 _returnvalue_5 "None" "KeepRelative" "KeepRelative" "SnapToTarget" true)
      (bind _returnvalue_7 (AddComponent|AddStaticMeshComponent true (Math|Transform|MakeTransform "0.000000,-200.000000,0.000000" (Math|Rotator|MakeRotator 0.0 0.0 (select (Variables|Default|GetLiftUp) 0.0 3e+01)) "1.000000,1.000000,1.000000")))
      (Transformation|AttachComponentToComponent _returnvalue_7 _returnvalue_5 "None" "KeepRelative" "KeepRelative" "SnapToTarget" true)
      (Variables|Default|SetDownDoors (Utilities|Array|MakeArray _returnvalue_7 _returnvalue_6)))
    (:then_2
      ;[1 1 1] Intermediate levels
      (for _index (range 1 (- (Variables|Default|GetNbFloors) 1))
        (AddComponent|AddStaticMeshComponent false (Math|Transform|MakeTransform (Math|Vector|MakeVector 0.0 0.0 (* _index 5e+02)) "0, 0, 0" "1.000000,1.000000,1.000000"))))
    (:then_3
      ;[1 1 1] Setup Top doors
      (bind _returnvalue_8 (AddComponent|AddStaticMeshComponent false (Math|Transform|MakeTransform (Math|Vector|MakeVector 0.0 0.0 (* (Variables|Default|GetNbFloors) 5e+02)) "0, 0, 0" "1.000000,1.000000,1.000000")))
      (bind _returnvalue_9 (AddComponent|AddStaticMeshComponent true (Math|Transform|MakeTransform "0.000000,-200.000000,0.000000" (Math|Rotator|MakeRotator 0.0 0.0 (select (Variables|Default|GetLiftUp) -3e+01 0.0)) "1.000000,1.000000,1.000000")))
      (Transformation|AttachComponentToComponent _returnvalue_9 _returnvalue_8 "None" "KeepRelative" "KeepRelative" "SnapToTarget" true)
      (bind _returnvalue_10 (AddComponent|AddStaticMeshComponent true (Math|Transform|MakeTransform "0.000000,-200.000000,0.000000" (Math|Rotator|MakeRotator 0.0 0.0 (select (Variables|Default|GetLiftUp) 3e+01 0.0)) "1.000000,1.000000,1.000000")))
      (Transformation|AttachComponentToComponent _returnvalue_10 _returnvalue_8 "None" "KeepRelative" "KeepRelative" "SnapToTarget" true)
      (Variables|Default|SetUpDoors (Utilities|Array|MakeArray _returnvalue_10 _returnvalue_9)))))

(fn ClearDoors)